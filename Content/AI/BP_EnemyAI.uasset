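; Deer enemy character that runs toward a target point, damages the player on contact and awards score when shot.
; SpawnSetting picks score, speed and scale from per-variant arrays, then starts an AI move that destroys the deer on arrival.
; First damage shows hit effects and a score popup, adds points, drops items for the first and last variants, and sends it fleeing until destroyed.
; Player contact removes a life and applies invincibility-dependent knockback.
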(event `SpawnSetting`
  (params (TargetPoint :type "Actor Object Reference") (StatusParam :type Integer) (RunawayPoint :type "Vector Structure"))
  (if (not (== StatusParam 5))
    (`ActorComponent.K2_DestroyComponent` (`self.P_ForgeDip_Firey`)))
  (set `self.StatusNum` StatusParam)
  (set `self.Score` (`|GetArrayItem` (`self.ScoreAry`) StatusParam))
  (set `self.RunawayPoint` RunawayPoint)
  (set `CharacterMovementComponent.MaxWalkSpeed` (`|GetArrayItem` (`self.SpeedAry`) StatusParam) (`self.CharacterMovement`))
  (`SceneComponent.SetWorldScale3D` (`self.CapsuleComponent`) (`|GetArrayItem` (`self.ScaleAry`) StatusParam))
  (`|AIMoveTo` (`CharacterMovementComponent.GetCharacterOwner` (`self.CharacterMovement`)) (`self.K2_GetActorLocation` TargetPoint) null 5.0 true
    (:`OnSuccess`
      (`self.K2_DestroyActor`)
      (`KismetSystemLibrary.PrintString` "鹿は目的地に着いた"))))

(event `self.ReceiveAnyDamage`
  (params (Damage :type "Float (single-precision)") (DamageType :type "DamageType Object Reference") (InstigatedBy :type "Controller Object Reference") (DamageCauser :type "Actor Object Reference"))
  (bind _returnvalue (`self.K2_GetActorLocation`))
  (set `CharacterMovementComponent.MaxWalkSpeed` 1000.0 (`self.CharacterMovement`))
  (if (not (`self.IsHit`))
    (set `self.IsHit` true)
    (`KismetSystemLibrary.PrintString` "鹿にヒット")
    (`GameplayStatics.SpawnEmitterAtLocation` "/Game/InfinityBladeEffects/Effects/FX_Combat_Ice/Impact/P_Impact_Ice.P_Impact_Ice" (`self.K2_GetActorLocation`) (struct) (1.7 1.7 1.7))
    (`AIBlueprintHelperLibrary.SimpleMoveToLocation` (`self.GetController`) (`self.RunawayPoint`))
    (`SceneComponent.SetVisibility` (`self.P_Stun_Stars_Base`) true false)
    (bind _returnvalue_2 (`|CreateWidget` "/Game/UI/Score.Score_C"))
    (bind _output_get (set `self.HUDReference` _returnvalue_2))
    (`UserWidget.AddToViewport` _output_get 0)
    (set `/Game/UI/Score.StartPosition` (`self.K2_GetActorLocation`) _returnvalue_2)
    (bind _output_get_2 (set `/Game/UI/Score.Score` (`self.Score`) _returnvalue_2))
    (bind _asfirst_person_character (cast `/Game/Blueprints/FirstPersonCharacter` (`GameplayStatics.GetPlayerCharacter` 0)))
    (set `/Game/Blueprints/FirstPersonCharacter.NowScore` (+ _output_get_2 (`/Game/Blueprints/FirstPersonCharacter.NowScore` _asfirst_person_character)) _asfirst_person_character)
    (`GameplayStatics.PlaySoundAtLocation` "/Game/Sounds/SE_DeerHit_Cue.SE_DeerHit_Cue" _returnvalue (struct) 1.0 1.0 0.0 null null null)
    (`GameplayStatics.PlaySoundAtLocation` "/Game/Sounds/SE_ScoreGet_Cue.SE_ScoreGet_Cue" _returnvalue (struct) 1.0 1.0 0.0 null null null)
    (if (== (`self.StatusNum`) (- (`KismetArrayLibrary.Array_Length` (`self.ScoreAry`)) 1))
      (`|SpawnActorFromClass` "/Game/Blueprints/Item_FireRateUpgrade.Item_FireRateUpgrade_C" (`KismetMathLibrary.MakeTransform` (.location (`self.GetTransform`)) (.rotation (`self.GetTransform`))) "Undefined" "OverrideRootScale" null null))
    (if (== (`self.StatusNum`) 0)
      (`|SpawnActorFromClass` "/Game/Blueprints/Item_Invincible.Item_Invincible_C" (`KismetMathLibrary.MakeTransform` (.location (`self.GetTransform`)) (.rotation (`self.GetTransform`))) "Undefined" "OverrideRootScale" null null))
    (`KismetSystemLibrary.Delay` 1.0)
    (`Widget.RemoveFromParent` _returnvalue_2)
    (`KismetSystemLibrary.Delay` 6.0)
    (`self.K2_DestroyActor`)
    (`KismetSystemLibrary.PrintString` "鹿は帰って行った")))

(event `self.ReceiveHit`
  (params (MyComp :type "PrimitiveComponent Object Reference") (Other :type "Actor Object Reference") (OtherComp :type "PrimitiveComponent Object Reference") (bSelfMoved :type Boolean) (HitLocation :type "Vector Structure") (HitNormal :type "Vector Structure") (NormalImpulse :type "Vector Structure") (Hit :type "HitResult Structure (by ref)"))
  (bind _asfirst_person_character (cast `/Game/Blueprints/FirstPersonCharacter` Other))
  (`/Game/Blueprints/FirstPersonCharacter.LifeDecrement` _asfirst_person_character)
  (if (not (and (`/Game/Blueprints/FirstPersonCharacter.IsHighInv` _asfirst_person_character) (`/Game/Blueprints/FirstPersonCharacter.IsInv` _asfirst_person_character)))
    (`CharacterMovementComponent.AddImpulse` (`Character.CharacterMovement` _asfirst_person_character) (* (* (- (`self.K2_GetActorLocation` _asfirst_person_character) (`self.K2_GetActorLocation`)) 500.0) (2.0 2.0 0.5)) false)))

(fn `UserConstructionScript`)