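; BP_EnemySpawn is a spawner actor that releases BP_EnemyAI enemies one at a time on a timed wave schedule.
; From BeginPlay, it loops through parallel arrays indexed by WaveCount for each delay and status parameter, spawning at its own transform with BT_Enemy.
; Each enemy receives the target point, status parameter and runaway location through SpawnSetting.
; The spawner destroys itself after the last array entry, and a failed cast halts the loop.
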(event `self.ReceiveBeginPlay`
  (`KismetSystemLibrary.Delay` (`|GetArrayItem` (`self.SpawnEnemyDurationAry`) (`self.WaveCount`)) :!label _label)
  (bind _returnvalue (`AIBlueprintHelperLibrary.SpawnAIFromClass` "/Game/AI/BP_EnemyAI.BP_EnemyAI_C" "/Game/AI/BT_Enemy.BT_Enemy" (`self.K2_GetActorLocation`) (`self.K2_GetActorRotation`) true null))
  (bind _asbp_enemy_ai (cast `/Game/AI/BP_EnemyAI` _returnvalue))
  (`/Game/AI/BP_EnemyAI.SpawnSetting` _asbp_enemy_ai (`self.TargetPoint`) (`|GetArrayItem` (`self.SpawnEnemyNumAry`) (`self.WaveCount`)) (`self.K2_GetActorLocation` (`self.RunawayPoints`)))
  (bind _output_get (set `self.WaveCount` (+ (`self.WaveCount`) 1)))
  (if (< _output_get (`KismetArrayLibrary.Array_Length` (`self.SpawnEnemyNumAry`)))
    (goto _label)
    (else
      (`self.K2_DestroyActor`))))

(fn `UserConstructionScript`)